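; ExplocubeHUD is the in-game HUD that owns the on-screen widget for ammo, money, health and an MC value.
; On BeginPlay it creates and caches the widget, switches to game-only input and copies current money from the game mode.
; Its events relay values to the widget: FireGun subtracts one from the passed ammo count, and health bar updates wait behind a short delay.
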(event Custom|CreateWidget)

(event Custom|SetHealth
  (params (Value :type Float%20%28double-precision%29))
  (Utilities|FlowControl|Delay 0.2)
  (Default|UpdateHealthBar (Variables|Default|GetAs%20WBP%20Explocube%20HUDWidget) Value))

(event Custom|SetAmmoText
  (params (AmmoText :type Integer))
  (bind _output_get (Variables|Default|SetCurrentAmmoAmount AmmoText))
  (Default|UpdateAmmo (Variables|Default|GetAs%20WBP%20Explocube%20HUDWidget) _output_get))

(event Custom|SetMoneyText
  (params (SetMoney :type Float%20%28double-precision%29))
  (Default|UpdateMoneyText (Variables|Default|GetAs%20WBP%20Explocube%20HUDWidget) SetMoney))

(event Custom|UpdateMCValueWidget
  (params (Hud :type Integer))
  (Default|SetMc (Variables|Default|GetAs%20WBP%20Explocube%20HUDWidget) (Utilities|Text|ToText(Integer) Hud)))

(event EventBeginPlay
  (bind _returnvalue (UserInterface|CreateWidget (Variables|Default|GetHUDWidget) (Game|Player|GetOwningPlayerController)))
  (bind _aswbp_explocube_hudwidget (Utilities|Casting|CastToWBP_ExplocubeHUDWidget _returnvalue))
  (bind _output_get (Variables|Default|SetAs%20WBP%20Explocube%20HUDWidget _aswbp_explocube_hudwidget))
  (UserInterface|Viewport|AddtoViewport _output_get 0)
  (Input|SetInputModeGameOnly (Game|GetPlayerController 0) false)
  (bind _asbp_explocube_game_mode (Utilities|Casting|CastToBP_ExplocubeGameMode (Game|GetGameMode)))
  (Variables|Default|SetCurrent%20Money (Variables|/Game/FirstPerson/Blueprints/BP_ExplocubeGameMode.BP_ExplocubeGameMode_C|GetCurrentMoney _asbp_explocube_game_mode)))

(event Collision|EventActorBeginOverlap
  (params (OtherActor :type Actor%20Object%20Reference)))

(event EventTick
  (params (DeltaSeconds :type Float%20%28single-precision%29)))

(event EventFireGun
  (params (RemainingAmmo :type Integer))
  (bind _output_get (Variables|Default|SetCurrentAmmoAmount (- RemainingAmmo 1)))
  (Default|UpdateAmmo (Variables|Default|GetAs%20WBP%20Explocube%20HUDWidget) _output_get))

(fn ConstructionScript)