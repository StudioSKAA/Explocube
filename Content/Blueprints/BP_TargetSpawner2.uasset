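; Target spawner actor that, on BeginPlay, spawns randomly chosen classes from CubesToSpawn at the transform of its Cube component.
; An inclusive loop from 0 to AntallKuber calls SelectCubes for each spawn.
; The Z offset divides the index by zero, so it adds no intended spacing between spawns.
; SelectCubes uses the array length as its inclusive random maximum, so it can index past the end.
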(event EventBeginPlay
  (bind _cube (Variables|Default|GetCube))
  (bind _returnvalue (Transformation|GetWorldTransform _cube))
  (bind (_location _rotation _scale) (Math|Transform|BreakTransform _returnvalue))
  (for _index (range 0 (Variables|Default|GetAntallKuber))
    (Game|SpawnActorfromClass (CallFunction|SelectCubes) (Math|Transform|MakeTransform (Math|Vector|MakeVector (.x _location) (.y _location) (+ (/ _index 0) (.z _location))) _rotation _scale) "Undefined" "SelectDefaultAtRuntime" 0 0)))

(fn ConstructionScript)

(fn SelectCubes
  (bind _cubestospawn (Variables|Default|GetCubesToSpawn))
  (return (Utilities|Array|Get(acopy) _cubestospawn (Math|Random|RandomIntegerinRange 0 (Utilities|Array|Length _cubestospawn)))))