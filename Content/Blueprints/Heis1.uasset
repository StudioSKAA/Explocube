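; Elevator actor that responds to an InBox event once the player's money meets a level minimum.
; InBox compares the Explocube game mode's CurrentMoney to LevelMinimumMoney, waits briefly, plays a ding at the actor and creates a level sequence player, with no Play call.
; BeginPlay sets that game mode reference to None, so the money check has no valid source here.
; A second sound node is never run.
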(event Custom|InBox
  (if (>= (Variables|/Game/FirstPerson/Blueprints/BP_ExplocubeGameMode.BP_ExplocubeGameMode_C|GetCurrentMoney (stale EventBeginPlay _output_get)) (Variables|Default|GetLevelMinimumMoney))
    (Utilities|FlowControl|Delay 3.0)
    (Audio|PlaySoundatLocation "/Game/ElevatorDING.ElevatorDING" (Transformation|GetActorLocation) "0, 0, 0" 1.0 1.0 0.0 0 0 0 0)
    (Sequencer|Player|CreateLevelSequencePlayer 0)))

(event EventBeginPlay
  (bind _output_get (Variables|Default|SetAs%20BP%20Explocube%20Game%20Mode 0)))

(fn ConstructionScript)