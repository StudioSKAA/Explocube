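; BP_Cube is a configurable physics cube for the Explocube game that explodes or implodes when hit.
; The construction script sets physics, optional debug radius sphere, material and radial impulse strength, negating the power for implosion.
; On hit it fires the impulse with particles and sound, optionally awards points through the game mode scaled by a game-instance multiplier, then optionally destroys itself.
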(event EventBeginPlay)

(event EventHit
  (bind _cube (Variables|Default|GetCube))
  (bind _returnvalue (Transformation|GetWorldTransform _cube))
  (Class|RadialForceComponent|FireImpulse (Variables|Default|GetRadialForce))
  (Effects|SpawnEmitteratLocation (Variables|Default|GetPartikkel%20System%20) (.location _returnvalue) (.rotation _returnvalue) "3.000000,3.000000,3.000000")
  (Audio|PlaySoundatLocation (Variables|Default|GetSound) (Transformation|GetWorldLocation (Variables|Default|GetCube)) "0, 0, 0" 1.0 1.0 0.0 0 0 0 0)
  (bind _asbp_explocube_game_mode (Utilities|Casting|CastToBP_ExplocubeGameMode (Game|GetGameMode)))
  (if (Variables|Default|GetGetPoints)
    (Default|AddPoints _asbp_explocube_game_mode (* (Variables|Default|GetPoints%20to%20Add) (Variables|/Game/Core/StudioSKAAGameInstance.StudioSKAAGameInstance_C|Getmc (.AsStudio%20SKAAGame%20Instance (Utilities|Casting|CastToStudioSKAAGameInstance (Game|GetGameInstance)))))))
  (if (Variables|Default|GetDestoryOnHit)
    (Actor|DestroyActor)))

(event EventTick
  (params (DeltaSeconds :type Float%20%28single-precision%29)))

(fn ConstructionScript
  (bind _implode (Variables|Default|GetImplode))
  (Physics|SetSimulatePhysics (Variables|Default|GetCube) (Variables|Default|GetSimulate%20Physics))
  (if (Variables|Default|GetDrawDebug)
    (Rendering|Debug|DrawDebugSphere (Transformation|GetActorLocation) (Variables|Default|GetRadius) 12 "(R=1.000000,G=1.000000,B=1.000000,A=1.000000)" 1.0 1.0))
  (Rendering|Material|SetMaterial (Variables|Default|GetCube) 0 (select _implode "/Game/Materials/MI_Heis.MI_Heis" "/Game/M_GlowingBox.M_GlowingBox"))
  (Variables|/Script/Engine.RadialForceComponent|SetImpulseStrength (Variables|Default|GetRadialForce) (Math|Float|SelectFloat (* (Math|Float|Absolute(Float) (Variables|Default|GetPower)) -1.0) (Variables|Default|GetPower) _implode)))