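; Boss cube enemy that shows its health as text and loses a point per BP_LeftShot hit.
; It loops between a swept rush at the player's saved position and a return to a fixed rest point, with timeline play rates picked at random for each attack.
; At zero health it explodes, animates global time dilation through a timeline, then spawns a shower of BP_Money and destroys itself.
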(event OnComponentHit(Cube)
  (params (HitComponent :type Primitive%20Component%20Object%20Reference) (OtherActor :type Actor%20Object%20Reference) (OtherComp :type Primitive%20Component%20Object%20Reference) (NormalImpulse :type Vector :default "0, 0, 0") (Hit :type Hit%20Result%20Structure%20%28by%20ref%29))
  (bind _returnvalue (Transformation|GetActorLocation))
  (Utilities|Casting|CastToBP_LeftShot OtherActor)
  (bind _output_get (Variables|Default|SetHealth (- (Variables|Default|GetHealth) 1)))
  (if (> (Variables|Default|GetHealth) 0)
    (Rendering|Components|TextRender|SetText (Variables|Default|GetTextRender) (Utilities|Text|ToText(Integer) _output_get))
    (else
      (Effects|SpawnEmitteratLocation "/Game/StarterContent/Particles/P_Explosion.P_Explosion" _returnvalue "0, 0, 0" "1000.000000,1000.000000,1000.000000")
      (Audio|SpawnSoundatLocation "/Game/StarterContent/Audio/Explosion01.Explosion01" _returnvalue "0, 0, 0" 1.0 1.0 0.0 0 0)
      (bind _newtrack_0 (Timeline|Timeline_0 Play)
        (:Update
          (Utilities|Time|SetGlobalTimeDilation _newtrack_0))
        (:Finished
          (for _index (range 0 200)
            (Game|SpawnActorfromClass "/Game/Blueprints/CubeTypes/BP_Money.BP_Money_C" (Math|Transform|MakeTransform (Transformation|GetActorLocation)) "Undefined" "MultiplyWithRoot" 0 0))
          (Actor|DestroyActor))))))

(event Custom|Attack
  (bind _output_get (Variables|Default|SetRandomNummer (Math|Random|RandomIntegerinRange 0 2)))
  (bind _alpha (|RushAttack (Utilities|Select :Index _output_get :Option%200 0.5 :Option%201 0.3 :Option%202 0.2))
    (:Update
      (|Rushing _alpha))
    (:Resting
      (Utilities|FlowControl|FlipFlop
        (:A
          (CallFunction|Resting (Utilities|Select :Index _output_get :Option%200 0.5 :Option%201 0.3 :Option%202 0.2)))
        (:B
          (CallFunction|Resting (Utilities|Select :Index _output_get :Option%200 0.5 :Option%201 0.3 :Option%202 0.2)))))))

(event Custom|Resting
  (params (RestingTime :type Float%20%28double-precision%29))
  (|NormalRest RestingTime))

(event Custom|CustomEvent)

(event Collision|EventActorBeginOverlap
  (params (OtherActor :type Actor%20Object%20Reference)))

(event EventTick
  (params (DeltaSeconds :type Float%20%28single-precision%29)))

(event EventBeginPlay
  (Rendering|Components|TextRender|SetText (Variables|Default|GetTextRender) (Utilities|Text|ToText(Integer) (Variables|Default|GetHealth)))
  (bind _asbp_first_person_character (Utilities|Casting|CastToBP_FirstPersonCharacter (Game|Player|GetPlayerPawn 0)))
  (Variables|Default|SetAs%20BP%20First%20Person%20Character _asbp_first_person_character)
  (Utilities|FlowControl|Delay 1.0)
  (CallFunction|Resting 1e+01)
  (CallFunction|Attack))

(fn ConstructionScript)