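; Test cube type Blueprint that sets off an explosion on every Tick, with no condition or delay.
; Each frame it fires the RadialForce impulse, then spawns a scaled-up P_Explosion emitter and plays Explosion01 at the Cube component's location.
; The Hit event is empty, BeginPlay is disabled, and the construction script only calls its parent.
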(event EventBeginPlay
  (|CallParentFunction) ; This node is disabled and will not be called.\nDrag off pins to build functionality.
)

(event EventTick
  (params (DeltaSeconds :type Float%20%28single-precision%29))
  (bind _cube (Variables|Default|GetCube))
  (bind _returnvalue (Transformation|GetWorldTransform _cube))
  (|CallParentFunction DeltaSeconds)
  (Class|RadialForceComponent|FireImpulse (Variables|Default|GetRadialForce))
  (Effects|SpawnEmitteratLocation "/Game/StarterContent/Particles/P_Explosion.P_Explosion" (.location _returnvalue) (.rotation _returnvalue) "3.000000,3.000000,3.000000")
  (Audio|PlaySoundatLocation "/Game/StarterContent/Audio/Explosion01.Explosion01" (.location _returnvalue) "0, 0, 0" 1.0 1.0 0.0 0 0 0 0))

(event EventHit)

(fn ConstructionScript
  (|CallParentFunction))