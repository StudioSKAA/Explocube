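; BP_Money is a money pickup cube that flies to the player and awards points.
; Overlap with the first-person character triggers a one-time flight, disabling gravity and using a timeline to lerp the cube from its current location toward the pawn's live position.
; When the timeline finishes, it adds points equal to the game instance's Mc value through the game mode, prints that amount, plays a sound and destroys itself.
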(event OnComponentBeginOverlap(Cube)
  (params (OverlappedComponent :type Primitive%20Component%20Object%20Reference) (OtherActor :type Actor%20Object%20Reference) (OtherComp :type Primitive%20Component%20Object%20Reference) (OtherBodyIndex :type Integer) (bFromSweep :type Boolean) (SweepResult :type Hit%20Result%20Structure%20%28by%20ref%29))
  (Utilities|Casting|CastToBP_FirstPersonCharacter OtherActor)
  (CallFunction|FlyTowardsPlayer))

(event Custom|FlyTowardsPlayer
  (bind _cube (Variables|Default|GetCube))
  (Utilities|FlowControl|DoOnce false
    (:Completed
      (Physics|SetEnableGravity (Variables|Default|GetCube) false)
      (bind _alpha (Timeline|Start%20lerp Play)
        (:Update
          (Transformation|SetWorldLocation _cube (Math|Vector|Lerp(Vector) (Transformation|GetWorldLocation _cube) (Transformation|GetActorLocation (Game|Player|GetPlayerPawn 0)) _alpha) false false))
        (:Finished
          (bind _asbp_explocube_game_mode (Utilities|Casting|CastToBP_ExplocubeGameMode (Game|GetGameMode)))
          (bind _asstudio_skaagame_instance (Utilities|Casting|CastToStudioSKAAGameInstance (Game|GetGameInstance)))
          (Default|AddPoints _asbp_explocube_game_mode (* 1.0 (Variables|/Game/Core/StudioSKAAGameInstance.StudioSKAAGameInstance_C|Getmc _asstudio_skaagame_instance)))
          (Development|PrintString (Utilities|String|ToString(Float) (* 1.0 (Variables|/Game/Core/StudioSKAAGameInstance.StudioSKAAGameInstance_C|Getmc _asstudio_skaagame_instance))))
          (Audio|PlaySound2D "/Game/audio/Money.Money" 1.0 1.0 0.0 0 0)
          (Actor|DestroyActor))))))

(event EventBeginPlay)

(event Collision|EventActorBeginOverlap
  (params (OtherActor :type Actor%20Object%20Reference)))

(fn ConstructionScript)