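; Base cube Blueprint, by its name the parent of the cube types, that fires a radial impulse when hit.
; The construction script copies the Power variable into the RadialForce component's ForceStrength, and the Hit event calls FireImpulse on that component.
; Power sets the continuous force rather than the ImpulseStrength that FireImpulse uses.
; BeginPlay and Tick are disabled stubs.
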(event EventBeginPlay
  (|CallParentFunction) ; This node is disabled and will not be called.\nDrag off pins to build functionality.
)

(event EventTick
  (params (DeltaSeconds :type Float%20%28single-precision%29))
  (|CallParentFunction DeltaSeconds) ; This node is disabled and will not be called.\nDrag off pins to build functionality.
)

(event EventHit
  (Class|RadialForceComponent|FireImpulse (Variables|Default|GetRadialForce)))

(fn ConstructionScript
  (|CallParentFunction)
  (Variables|/Script/Engine.RadialForceComponent|SetForceStrength (Variables|Default|GetRadialForce) (Variables|Default|GetPower)))