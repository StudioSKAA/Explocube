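; BP_Store is a store the player enters and leaves by pressing Enter while its Box trigger allows it.
; A FlipFlop in Interact toggles the game mode's InShop flag and blends the camera between the store and player pawn.
; Entering disables character movement and shows the cursor, with Block ignoring input during the delay.
; Leaving restores walking after a delay and hides the cursor, without setting Block.
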(event OnComponentBeginOverlap(Box)
  (params (OverlappedComponent :type Primitive%20Component%20Object%20Reference) (OtherActor :type Actor%20Object%20Reference) (OtherComp :type Primitive%20Component%20Object%20Reference) (OtherBodyIndex :type Integer) (bFromSweep :type Boolean) (SweepResult :type Hit%20Result%20Structure%20%28by%20ref%29))
  (Variables|Default|SetTillat_å_gå_inn true))

(event OnComponentEndOverlap(Box)
  (params (OverlappedComponent :type Primitive%20Component%20Object%20Reference) (OtherActor :type Actor%20Object%20Reference) (OtherComp :type Primitive%20Component%20Object%20Reference) (OtherBodyIndex :type Integer))
  (Variables|Default|SetTillat_å_gå_inn false))

(event Custom|Interact
  (bind _returnvalue (Game|GetPlayerController 0))
  (Utilities|FlowControl|FlipFlop
    (:A
      (CallFunction|SetinStore true)
      (Variables|Default|SetBlock true)
      (Game|Player|SetViewTargetwithBlend (Game|GetPlayerController 0) self 0.0 "VTBlend_Cubic" 1.2 false)
      (CallFunction|SetMovementMode "MOVE_None")
      (Utilities|FlowControl|Delay 1.0)
      (Variables|Default|SetBlock false)
      (Variables|/Script/Engine.PlayerController|SetbShowMouseCursor _returnvalue true))
    (:B
      (CallFunction|SetinStore false)
      (Game|Player|SetViewTargetwithBlend (Game|GetPlayerController 0) (Game|Player|GetPlayerPawn 0) 0.0 "VTBlend_Cubic" 1.2 false)
      (Utilities|FlowControl|Delay 1.0)
      (CallFunction|SetMovementMode "MOVE_Walking")
      (Variables|/Script/Engine.PlayerController|SetbShowMouseCursor _returnvalue false))))

(event EventBeginPlay)

(event Collision|EventActorBeginOverlap
  (params (OtherActor :type Actor%20Object%20Reference)))

(event EventTick
  (params (DeltaSeconds :type Float%20%28single-precision%29)))

(event Input|KeyboardEvents|Enter
  (params (Key :type Key%20Structure :default "None"))
  (:Pressed
    (if (Variables|Default|GetTillat_å_gå_inn)
      (if (not (Variables|Default|GetBlock))
        (CallFunction|Interact)))))

(fn ConstructionScript)

(fn SetMovementMode
  (params (NewMovementMode :type EMovementMode%20Enum :default "MOVE_None"))
  (bind _asbp_first_person_character (Utilities|Casting|CastToBP_FirstPersonCharacter (Game|Player|GetPlayerPawn 0)))
  (Pawn|Components|CharacterMovement|SetMovementMode (Variables|/Script/Engine.Character|GetCharacterMovement _asbp_first_person_character) NewMovementMode 0))

(fn SetinStore
  (params (In%20shop :type Boolean))
  (bind _asbp_explocube_game_mode (Utilities|Casting|CastToBP_ExplocubeGameMode (Game|GetGameMode)))
  (Variables|/Game/FirstPerson/Blueprints/BP_ExplocubeGameMode.BP_ExplocubeGameMode_C|SetIn%20shop _asbp_explocube_game_mode In%20shop))