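; Elevator actor for Explocube that runs its sequence when the player has enough money for the level.
; Any overlap with its Box reads CurrentMoney from BP_ExplocubeGameMode and compares it to LevelMinimumMoney.
; On success it plays a ding, starts the assigned level sequence, then pauses it after a fixed delay.
; Disconnected leftovers reference other audio, level-instance loading and a level selection menu.
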(event OnComponentBeginOverlap(Box)
  (params (OverlappedComponent :type Primitive%20Component%20Object%20Reference) (OtherActor :type Actor%20Object%20Reference) (OtherComp :type Primitive%20Component%20Object%20Reference) (OtherBodyIndex :type Integer) (bFromSweep :type Boolean) (SweepResult :type Hit%20Result%20Structure%20%28by%20ref%29))
  (CallFunction|InBox))

(event Custom|InBox
  (bind _asbp_explocube_game_mode (Utilities|Casting|CastToBP_ExplocubeGameMode (Game|GetGameMode)))
  (bind _output_get (Variables|Default|SetAs%20BP%20Explocube%20Game%20Mode _asbp_explocube_game_mode))
  (if (>= (Variables|/Game/FirstPerson/Blueprints/BP_ExplocubeGameMode.BP_ExplocubeGameMode_C|GetCurrentMoney _output_get) (Variables|Default|GetLevelMinimumMoney))
    (Audio|PlaySoundatLocation "/Game/ElevatorDING.ElevatorDING" (Transformation|GetActorLocation) "0, 0, 0" 1.0 1.0 0.0 0 0 0 0)
    (bind _returnvalue (Sequencer|Player|CreateLevelSequencePlayer (Variables|Default|GetLevel%20sequense)))
    (Sequencer|Player|Play _returnvalue :!class /Script/MovieScene.MovieSceneSequencePlayer)
    (Utilities|FlowControl|Delay 5.2)
    (Sequencer|Player|Pause _returnvalue)))

(event EventBeginPlay)

(fn ConstructionScript)