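; BADHEIS is an elevator actor that ends the level once the player has enough money.
; When its box trigger is overlapped, it compares the Explocube game mode's CurrentMoney against a level minimum.
; On success it plays a ding and a level sequence, pauses it after a fixed delay, then shows a widget with the mouse cursor and UI-only input.
; Leftover sound and level-instance loading nodes are unconnected.
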(event OnComponentBeginOverlap(Box)
  (params (OverlappedComponent :type Primitive%20Component%20Object%20Reference) (OtherActor :type Actor%20Object%20Reference) (OtherComp :type Primitive%20Component%20Object%20Reference) (OtherBodyIndex :type Integer) (bFromSweep :type Boolean) (SweepResult :type Hit%20Result%20Structure%20%28by%20ref%29))
  (CallFunction|InBox))

(event Custom|InBox
  (bind _returnvalue (Game|GetPlayerController 0))
  (bind _asbp_explocube_game_mode (Utilities|Casting|CastToBP_ExplocubeGameMode (Game|GetGameMode)))
  (bind _output_get (Variables|Default|SetAs%20BP%20Explocube%20Game%20Mode _asbp_explocube_game_mode))
  (if (>= (Variables|/Game/FirstPerson/Blueprints/BP_ExplocubeGameMode.BP_ExplocubeGameMode_C|GetCurrentMoney _output_get) (Variables|Default|GetLevelMinimumMoney))
    (Audio|PlaySoundatLocation "/Game/ElevatorDING.ElevatorDING" (Transformation|GetActorLocation) "0, 0, 0" 1.0 1.0 0.0 0 0 0 0)
    (bind _returnvalue_2 (Sequencer|Player|CreateLevelSequencePlayer (Variables|Default|GetLevel%20sequense)))
    (Sequencer|Player|Play _returnvalue_2 :!class /Script/MovieScene.MovieSceneSequencePlayer)
    (Utilities|FlowControl|Delay 5.2)
    (Sequencer|Player|Pause _returnvalue_2)
    (bind _returnvalue_3 (UserInterface|CreateWidget "/Game/Menulevelblueprints/DONTREFERENCETHIS.DONTREFERENCETHIS_C"))
    (UserInterface|Viewport|AddtoViewport _returnvalue_3 0)
    (Variables|/Script/Engine.PlayerController|SetbShowMouseCursor _returnvalue true)
    (Input|SetInputModeUIOnly _returnvalue 0 "DoNotLock" false)))

(event EventBeginPlay)

(fn ConstructionScript)