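; BP_SnowmanCharacter is a snowman character that fires BP_RightShot projectiles automatically on a fast looping timer started at BeginPlay.
; Each shot spawns at the snowman's transform, after which the snowman rotates to face the BP_Exploding_Points actor found in the level.
; The projectile's sphere then receives a fixed impulse along world X, so its launch direction does not follow that aim.
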(event Custom|Shoot
  (bind _returnvalue (Transformation|GetActorTransform))
  (bind _returnvalue_2 (Actor|GetActorOfClass "/Game/Blueprints/CubeTypes/BP_Exploding_Points.BP_Exploding_Points_C"))
  (bind _returnvalue_3 (Game|SpawnActorfromClass "/Game/FirstPerson/Blueprints/BP_RightShot.BP_RightShot_C" (Math|Transform|MakeTransform (.location _returnvalue) (.rotation _returnvalue) (.scale _returnvalue)) "Undefined" "MultiplyWithRoot" 0 0))
  (Transformation|SetActorRotation (Math|Rotator|FindLookatRotation (Transformation|GetActorLocation) (Transformation|GetActorLocation _returnvalue_2)))
  (Physics|AddImpulse (Variables|/Game/FirstPerson/Blueprints/BP_ProjectileParent.BP_ProjectileParent_C|GetSphere _returnvalue_3) "100000.000000,0.000000,0.000000" "None" false))

(event EventBeginPlay
  (Utilities|Time|SetTimerbyEvent (delegate Custom|Shoot) 0.2 true))

(event Collision|EventActorBeginOverlap
  (params (OtherActor :type Actor%20Object%20Reference)))

(event EventTick
  (params (DeltaSeconds :type Float%20%28single-precision%29)))

(fn ConstructionScript)