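; Base Blueprint for purchasable items in Explocube, bought by clicking the actor.
; A click passes the item's price and itself to the game mode's ChangeCurensy, while CanAfford and CannotAfford events play the matching purchase sounds.
; The construction script applies the static mesh, then clears either that mesh variable or the SKFPGun skeletal mesh, depending on whether SkeletalMesh is set.
; Try-Buy and the bound OnClicked_Event handler are empty.
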(event Custom|Try-Buy)

(event Custom|OnClicked_Event
  (params (TouchedActor :type Actor%20Object%20Reference) (ButtonPressed :type Key%20Structure :default "None")))

(event Custom|CanAfford
  (Audio|PlaySound2D (Variables|Default|GetBuy-sound) 1.0 1.0 0.0 0 0))

(event Custom|CannotAfford
  (Audio|PlaySound2D (Variables|Default|GetCantAffordSound) 1.0 1.0 0.0 0 0))

(event EventBeginPlay
  (EventDispatchers|BindEventtoOnClicked (delegate Custom|OnClicked_Event)))

(event MouseInput|EventActorOnClicked
  (params (ButtonPressed :type Key%20Structure :default "None"))
  (bind _asbp_explocube_game_mode (Utilities|Casting|CastToBP_ExplocubeGameMode (Game|GetGameMode)))
  (Default|ChangeCurensy _asbp_explocube_game_mode (Variables|Default|GetPrice) self))

(fn ConstructionScript
  (Components|StaticMesh|SetStaticMesh (Variables|Default|Getitem_Mesh) (Variables|Default|GetstaticMesh))
  (if (Variables|Default|GetSkeletalMesh)
    (Variables|Default|SetstaticMesh 0)
    (else
      (Components|SkeletalMesh|SetSkeletalMeshAsset (Variables|Default|GetSK_FPGun) 0))))