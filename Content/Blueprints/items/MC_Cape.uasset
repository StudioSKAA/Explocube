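; MC_Cape is a clickable item Blueprint for a cape, tied to the MC value stored in the StudioSKAA game instance.
; On click, it runs the parent click logic and sets MC to MCBronse, unless MC already exceeds that value.
; A custom MC_Cape event triggers the same click handler, calls MCCape, then moves a component to a fixed relative location.
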(event Custom|MC_Cape
  (CallFunction|OnClickedEvent 0 "LeftMouseButton")
  (CallFunction|MCCape)
  (Components|MoveComponentTo 0 "-70.642334,-4112.845678,185.251805" "0, 0, 0" false false 0.2 false))

(event Collision|EventActorBeginOverlap
  (params (OtherActor :type Actor%20Object%20Reference)))

(event EventTick
  (params (DeltaSeconds :type Float%20%28single-precision%29)))

(event EventOnClickedEvent
  (params (TouchedActor :type Actor%20Object%20Reference) (ButtonPressed :type Key%20Structure :default "None"))
  (bind _returnvalue (Game|GetGameInstance))
  (bind _asstudio_skaagame_instance (Utilities|Casting|CastToStudioSKAAGameInstance _returnvalue))
  (if (not (< (Variables|Default|GetMC_Bronse) (Variables|/Game/Core/StudioSKAAGameInstance.StudioSKAAGameInstance_C|Getmc _asstudio_skaagame_instance)))
    (|CallParentFunction TouchedActor ButtonPressed)
    (Default|SetMC _asstudio_skaagame_instance (Variables|Default|GetMC_Bronse))))

(fn ConstructionScript
  (|CallParentFunction))