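; BP_Grenade is a clickable grenade item meant to add to the player's grenade count.
; The Capsule's OnClicked event casts to MyPlayerController, increments Grenades and prints a debug "Hello".
; The cast takes the clicked component rather than a controller, so the increment and print should not execute.
; An actor-level OnClicked binding is left unconnected with an empty handler, and the default events are unused.
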(event OnClicked(Capsule)
  (params (TouchedComponent :type Primitive%20Component%20Object%20Reference) (ButtonPressed :type Key%20Structure :default "None"))
  (bind _asmy_player_controller (Utilities|Casting|CastToMyPlayerController TouchedComponent))
  (Variables|/Game/MyPlayerController.MyPlayerController_C|SetGrenades _asmy_player_controller (+ (Variables|/Game/MyPlayerController.MyPlayerController_C|GetGrenades _asmy_player_controller) 1))
  (Development|PrintString "Hello"))

(event Custom|OnClicked_Event
  (params (TouchedActor :type Actor%20Object%20Reference) (ButtonPressed :type Key%20Structure :default "None")))

(event EventBeginPlay
  (|CallParentFunction) ; This node is disabled and will not be called.\nDrag off pins to build functionality.
)

(event Collision|EventActorBeginOverlap
  (params (OtherActor :type Actor%20Object%20Reference)))

(event EventTick
  (params (DeltaSeconds :type Float%20%28single-precision%29)))

(fn ConstructionScript
  (|CallParentFunction))