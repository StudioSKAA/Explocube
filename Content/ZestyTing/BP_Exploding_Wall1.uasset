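; BP_Exploding_Wall1 is a target wall that awards a range point when a projectile hits it.
; A hit on its Cube by a BP_ProjectileParent finds the Point_counter actor and calls AddRengePoint.
; On BeginPlay it saves its location, then Telleport overwrites that variable with a fixed X and random Y and Z.
; The graph shows no explosion or actual move, and hits do not re-trigger Telleport.
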(event OnComponentHit(Cube)
  (params (HitComponent :type Primitive%20Component%20Object%20Reference) (OtherActor :type Actor%20Object%20Reference) (OtherComp :type Primitive%20Component%20Object%20Reference) (NormalImpulse :type Vector :default "0, 0, 0") (Hit :type Hit%20Result%20Structure%20%28by%20ref%29))
  (Utilities|Casting|CastToBP_ProjectileParent OtherActor)
  (bind _returnvalue (Actor|GetActorOfClass "/Game/ZestyTing/Point_counter.Point_counter_C"))
  (Default|AddRengePoint _returnvalue))

(event Custom|Telleport
  (Variables|Default|SetLocation (Math|Vector|MakeVector 2194.211043 (Math|Random|RandomFloatinRange 555.711424 1224.515803) (Math|Random|RandomFloatinRange 0.0 2761.948933))))

(event EventBeginPlay
  (Variables|Default|SetLocation (Transformation|GetActorLocation))
  (CallFunction|Telleport))

(event EventTick
  (params (DeltaSeconds :type Float%20%28single-precision%29))
  (|CallParentFunction DeltaSeconds) ; This node is disabled and will not be called.\nDrag off pins to build functionality.
)

(fn ConstructionScript
  (|CallParentFunction))