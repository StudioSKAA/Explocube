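; BP_Cube is a cube actor with a configurable physics-simulation toggle and Radius, Power and Implode variables, which suggest a radial force setup.
; Its construction script applies the physics toggle to the Cube component and, when DrawDebug is on, draws a debug sphere at the actor's location.
; Implode negates Power only inside that debug branch.
; The event graph is empty, and nothing in this file applies Power.
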(event EventBeginPlay)

(event EventHit)

(event EventTick
  (params (DeltaSeconds :type Float%20%28single-precision%29)))

(fn ConstructionScript
  (Physics|SetSimulatePhysics (Variables|Default|GetCube) (Variables|Default|GetSimulate%20Physics))
  (if (Variables|Default|GetDrawDebug)
    (Rendering|Debug|DrawDebugSphere (Transformation|GetActorLocation) (Variables|Default|GetRadius) 12 "(R=1.000000,G=1.000000,B=1.000000,A=1.000000)" 1.0 1.0)
    (if (Variables|Default|GetImplode)
      (Variables|Default|SetPower (* (Variables|Default|GetPower) -1.0)))))