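; BP_CubeRevised is an Explocube cube actor that explodes with an effect and sound when hit.
; If flagged to destroy on hit, it awards points through BP_ExplocubeGameMode and destroys itself.
; The construction script sets Cube physics simulation, optionally draws a debug radius sphere, and negates Power when Implode is set.
; Power and Radius drive no force in these graphs.
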(event EventBeginPlay)

(event EventHit
  (bind _cube (Variables|Default|GetCube))
  (bind _returnvalue (Transformation|GetWorldTransform _cube))
  (Effects|SpawnEmitteratLocation "/Game/StarterContent/Particles/P_Explosion.P_Explosion" (.location _returnvalue) (.rotation _returnvalue) "3.000000,3.000000,3.000000")
  (Audio|PlaySoundatLocation (Variables|Default|GetSoundToPlay) (.location _returnvalue) "0, 0, 0" 1.0 1.0 0.0 0 0 0 0)
  (bind _asbp_explocube_game_mode (Utilities|Casting|CastToBP_ExplocubeGameMode (Game|GetGameMode)))
  (if (Variables|Default|GetDestoryOnHit)
    (Default|AddPoints _asbp_explocube_game_mode (Variables|Default|GetPoints%20to%20Add))
    (Actor|DestroyActor)))

(event EventTick
  (params (DeltaSeconds :type Float%20%28single-precision%29)))

(fn ConstructionScript
  (Utilities|FlowControl|Sequence
    (:then_0
      (Physics|SetSimulatePhysics (Variables|Default|GetCube) (Variables|Default|GetSimulate%20Physics)))
    (:then_1
      (if (Variables|Default|GetDrawDebug)
        (Rendering|Debug|DrawDebugSphere (Transformation|GetActorLocation) (Variables|Default|GetRadius) 12 "(R=1.000000,G=1.000000,B=1.000000,A=1.000000)" 1.0 1.0)))
    (:then_2
      (Variables|Default|SetPower (* (Variables|Default|GetPower) (Math|Integer|SelectInt -1 1 (Variables|Default|GetImplode)))))))